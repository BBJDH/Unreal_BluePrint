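; Enemy Blueprint that links the character's state changes to its AI behavior.
; On BeginPlay it runs the parent logic, then binds a handler to the StateComponent's state-type change event.
; When the new state is Hitted, the handler writes a fixed behavior enum value to the Behavior key on the AI controller's Blackboard.
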(event Custom|OnStateTypeChanged_AI
  (params (InPrevType :type EStateType%20Enum :default "NewEnumerator0") (InNewType :type EStateType%20Enum :default "NewEnumerator0"))
  (switch Utilities|FlowControl|Switch|SwitchonEStateType InNewType
    (:NewEnumerator5
      (AI|Components|Blackboard|SetValueasEnum (Variables|/Script/AIModule.AIController|GetBlackboard (AI|GetAIController self)) (Utilities|Name|MakeLiteralName "Behavior") (Utilities|Enum|LiteralenumEBehaior_Type "NewEnumerator4")))))

(event EventBeginPlay
  (|CallParentFunction)
  (EventDispatchers|BindEventtoOnStateTypeChanged (Variables|Default|GetStateComponent) (delegate Custom|OnStateTypeChanged_AI)))

(fn ConstructionScript
  (|CallParentFunction))