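; Enemy character that takes hits, shows a floating health bar scaled by camera distance and hidden when occluded, and dies with a montage.
; Damaged stores HitData and sets StateComponent's hit state, whose change event subtracts health and branches to death or reaction.
; HitData drives montage, knockback, particles, sound and camera shake, alongside a red material flash.
; Hit stop slows CustomTimeDilation on pawns or movable-mesh actors, restored by timer.
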(event Custom|Dead
  (Collision|SetCollisionEnabled (Variables|Collision|GetCapsuleComponent) "NoCollision")
  (Animation|PlayAnimMontage "/Game/Character/Montages/Comon/Enemy_DeadFall1_Montage.Enemy_DeadFall1_Montage" 1.0 "None"))

(event Custom|End_Dead
  (Actor|DestroyActor))

(event Custom|OnStateTypeChanged_Event
  (params (InPrevType :type EStateType%20Enum :default "NewEnumerator0") (InNewType :type EStateType%20Enum :default "NewEnumerator0"))
  (switch Utilities|FlowControl|Switch|SwitchonEStateType InNewType
    (:NewEnumerator5
      (CallFunction|Hitted))))

(event Custom|Hitted
  (|SetDamage (.Damage (Utilities|Struct|BreakFHitData (Variables|Hitted|GetHitData)))
    (:Dead
      (CallFunction|Dead))
    (:hitted
      (Game|Damage|ApplyDamage))))

(event EventDamaged
  (params (Attacker :type Character%20Object%20Reference) (Causer :type Actor%20Object%20Reference) (HitData :type F%20Hit%20Data%20Structure))
  (Variables|Default|SetAttacker Attacker)
  (Variables|Hitted|SetCauser Causer)
  (Variables|Hitted|SetHitData HitData)
  (Default|SetHittedMode (Variables|Default|GetStateComponent)))

(event EventTick
  (params (DeltaSeconds :type Float%20%28single-precision%29))
  (bind _returnvalue (Game|GetPlayerCameraManager 0))
  (bind _healthbar (Variables|Default|GetHealthBar))
  (bind _aswb_health_bar (Utilities|Casting|CastToWB_HealthBar (UserInterface|GetUserWidgetObject (Variables|Default|GetHealthBar))))
  (Widget|Transform|SetRenderScale _aswb_health_bar (* (Math|Vector2D|MakeVector2D 1.0 1.0) (/ 1e+03 (Transformation|GetDistanceTo _returnvalue))))
  (bind _outhit (Collision|LineTraceByChannel (Camera|GetCameraLocation _returnvalue) (Transformation|GetWorldLocation (Variables|Default|GetHealthBar)) "TraceTypeQuery1" false 0 "None"))
  (if (.bBlockingHit (Collision|BreakHitResult _outhit))
    (Rendering|SetVisibility _healthbar false false)
    (else
      (Rendering|SetVisibility _healthbar true true))))

(event EventBeginPlay
  (Utilities|FlowControl|Sequence
    (:then_0
      (for _array_element (Rendering|Material|GetMaterials (Variables|Character|GetMesh))
        (bind _returnvalue (Rendering|Material|CreateDynamicMaterialInstance _array_element "None" "None" :!class /Script/Engine.KismetMaterialLibrary))
        (bind _returnvalue_2 (Utilities|Array|Add (Variables|Default|GetMaterials) _returnvalue))
        (Rendering|Material|SetMaterial (Variables|Character|GetMesh) _returnvalue_2 _returnvalue)))
    (:then_1
      (EventDispatchers|AssignOnStateTypeChanged (Variables|Default|GetStateComponent) (delegate Custom|OnStateTypeChanged_Event)))
    (:then_2
      (Variables|Default|SetHealth (Variables|Default|GetMaxHealth))
      (CallFunction|UpdateHealthBar))))

(fn ConstructionScript)

(fn UpdateHealthBar
  (bind _aswb_health_bar (Utilities|Casting|CastToWB_HealthBar (UserInterface|GetUserWidgetObject (Variables|Default|GetHealthBar))))
  (Default|UpdateHealthBar _aswb_health_bar (Variables|Default|GetHealth) (Variables|Default|GetMaxHealth))
  (Default|UpdateControllerName _aswb_health_bar (Utilities|String|StringToName (Utilities|GetObjectName (Pawn|GetController)))))

(event Custom|RestoreTImeDelation
  (bind _delationactors (Variables|Default|GetDelationActors))
  (for _array_element _delationactors
    (Variables|/Script/Engine.Actor|SetCustomTimeDilation _array_element 1.0))
  (Utilities|Array|Clear _delationactors))